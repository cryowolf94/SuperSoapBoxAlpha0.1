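; Tutorial game mode that opens a TutorialSubMenu with a mouse cursor and offers single-player and local multiplayer setup events.
; Single player spawns and possesses a vehicle at a spawn point and binds its overlap event.
; Multiplayer creates extra local players, spawning vehicles for controllers 0 and 1 inside that loop, without overlap binding.
; Both setups then spawn and initialise a TutorialPlayerManager, whose phases the game mode can advance.
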(event Custom|SpawnManagers
  ;[0.1028 0 1] init tut manager spawn location
  (bind _returnvalue (Game|SpawnActorfromClass "/Game/VehicleAdvBP/Blueprints/TutorialBP/TutorialPlayerManager.TutorialPlayerManager_C" (Math|Transform|MakeTransform "0, 0,10000.000000" "0, 0, 0" "1,1,1") "AlwaysSpawn" self 0))
  (bind _output_get (Variables|Default|Settut%20manager%20ref _returnvalue))
  (Default|InitMnager _output_get))

(event Custom|set-up%20multiplayer
  ;[0 0.07942 1] init process for level
  (CallFunction|Multiplayer)
  (CallFunction|SpawnManagers))

(event Custom|Multiplayer
  ;[1 1 1] multiplayer funshionalty
  (for _index (range 1 (- (Variables|Default|GetNumberOfPlayersToSpawn) 1))
    (bind _returnvalue (Class|GameplayStatics|CreatePlayer _index))
    (bind _asplayer_controller_proto (Utilities|Casting|CastToPlayerControllerPROTO _returnvalue))
    (Variables|/Game/VehicleAdvBP/Blueprints/Players/PlayerControllerPROTO.PlayerControllerPROTO_C|SetPlayerID _asplayer_controller_proto _index)
    ;[1 1 1] put in separate functions
    (bind _outactors (Actor|GetAllActorsOfClass "/Game/VehicleAdvBP/Blueprints/Players/SpawnPoints/Player1SPN.Player1SPN_C"))
    (bind _returnvalue_2 (Game|SpawnActorfromClass "/Game/VehicleAdvBP/Blueprints/Players/PlayerVechilePROTO.PlayerVechilePROTO_C" (Transformation|GetActorTransform (Utilities|Array|Get(acopy) _outactors)) "AlwaysSpawn" self 0))
    (Pawn|Possess (Game|GetPlayerController 0) _returnvalue_2)
    (bind _outactors_2 (Actor|GetAllActorsOfClass "/Game/VehicleAdvBP/Blueprints/Players/SpawnPoints/Player2SPN.Player2SPN_C"))
    (bind _returnvalue_3 (Game|SpawnActorfromClass "/Game/VehicleAdvBP/Blueprints/Players/PlayerVechilePROTO.PlayerVechilePROTO_C" (Transformation|GetActorTransform (Utilities|Array|Get(acopy) _outactors_2)) "AlwaysSpawn" self 0))
    (Pawn|Possess (Game|GetPlayerController 1) _returnvalue_3)))

(event Custom|#
  ;[1 0.1254 0] dident work
)

(event Custom|setup%20single%20player
  ;[0 0.07942 1] init process for level
  (CallFunction|SpawnSinglePlayer)
  (CallFunction|SpawnManagers))

(event Custom|SpawnSinglePlayer
  ;[0 0.07942 1] SpawnPlayer
  (bind _outactors (Actor|GetAllActorsOfClass "/Game/VehicleAdvBP/Blueprints/Players/SpawnPoints/ParentPlayerSpawnPoint.ParentPlayerSpawnPoint_C"))
  (bind _returnvalue (Game|SpawnActorfromClass "/Game/VehicleAdvBP/Blueprints/Players/PlayerVechilePROTO.PlayerVechilePROTO_C" (Transformation|GetActorTransform (Utilities|Array|Get(acopy) _outactors)) "AlwaysSpawn" self 0))
  (Pawn|Possess (Game|GetPlayerController 0) _returnvalue)
  ;[0.164 0 1] finally observer works!!!!
  (EventDispatchers|BindEventtoOverlapptedColl _returnvalue (delegate Custom|####)))

(event Custom|####
  ;[0.164 0 1] finally observer works!!!!
  (Default|SetNextPhase (Variables|Default|Gettut%20manager%20ref)))

(event EventBeginPlay
  ;[0 0.07942 1] init process for level
  (bind _returnvalue (UserInterface|CreateWidget "/Game/VehicleAdvBP/Blueprints/MenuAndUI/TutorialSubMenu.TutorialSubMenu_C" (Game|GetPlayerController 0) self))
  (UserInterface|Viewport|AddtoViewport _returnvalue 0)
  (Variables|/Script/Engine.PlayerController|SetbShowMouseCursor (Game|GetPlayerController 0) true))

(fn ConstructionScript)