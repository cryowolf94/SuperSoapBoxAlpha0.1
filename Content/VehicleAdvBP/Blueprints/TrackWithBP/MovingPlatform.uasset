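; Moving track platform for the vehicle game that shifts its static mesh along relative Y from BeginPlay.
; A timeline drives the motion, with its track output fed as the Lerp start value toward a fixed target and SpeedOfLife as the alpha.
; Box overlaps set and clear IsPlayerOnTrack on PlayerVechilePROTO.
; Reverse and delayed-reset logic is left unfinished or disconnected.
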(event OnComponentBeginOverlap(Box)
  (params (OverlappedComponent :type Primitive%20Component%20Object%20Reference) (OtherActor :type Actor%20Object%20Reference) (OtherComp :type Primitive%20Component%20Object%20Reference) (OtherBodyIndex :type Integer) (bFromSweep :type Boolean) (SweepResult :type Hit%20Result%20Structure%20%28by%20ref%29))
  ;[1 1 1] Comment
  (bind _asplayer_vechile_proto (Utilities|Casting|CastToPlayerVechilePROTO OtherActor))
  (Variables|/Game/VehicleAdvBP/Blueprints/Players/PlayerVechilePROTO.PlayerVechilePROTO_C|SetIsPlayerOnTrack _asplayer_vechile_proto true))

(event OnComponentEndOverlap(Box)
  (params (OverlappedComponent :type Primitive%20Component%20Object%20Reference) (OtherActor :type Actor%20Object%20Reference) (OtherComp :type Primitive%20Component%20Object%20Reference) (OtherBodyIndex :type Integer))
  ;[1 1 1] Comment
  (bind _asplayer_vechile_proto (Utilities|Casting|CastToPlayerVechilePROTO OtherActor))
  (Variables|/Game/VehicleAdvBP/Blueprints/Players/PlayerVechilePROTO.PlayerVechilePROTO_C|SetIsPlayerOnTrack _asplayer_vechile_proto false))

(event Custom|reset
  (Utilities|FlowControl|DoOnce false) ; enters at Reset
)

(event Custom|Revserse)

(event EventBeginPlay
  (bind _newtrack_1 (Timeline|Timeline_0 Play)
    (:Update
      (Transformation|SetRelativeLocationAndRotation (Variables|Default|GetStaticMesh) (Math|Vector|MakeVector 0.0 (Math|Float|Lerp _newtrack_1 1e+02 (Variables|Default|GetSpeedOfLife)) 0.0) "0, 0, 0" false false))))

(fn ConstructionScript)