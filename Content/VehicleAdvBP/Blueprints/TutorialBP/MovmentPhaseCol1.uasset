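; Tutorial trigger volume that checks whether the player vehicle has used all movement controls before the tutorial moves on.
; When a PlayerVechilePROTO leaves the box, it requires the WS, AD, handbrake and camera movement flags together.
; Success calls CallOverlapptedColl on the vehicle; failure teleports it to the first ParentPlayerSpawnPoint found and prints a retry message.
; The parent reference from INIT and older manager-notification nodes are unused by the live path.
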(event OnComponentEndOverlap(Box)
  (params (OverlappedComponent :type Primitive%20Component%20Object%20Reference) (OtherActor :type Actor%20Object%20Reference) (OtherComp :type Primitive%20Component%20Object%20Reference) (OtherBodyIndex :type Integer))
  ;[0.06146 0 1] checking to see if all movement conditions wher met
  (bind _asplayer_vechile_proto (Utilities|Casting|CastToPlayerVechilePROTO OtherActor))
  (bind _output_get (Variables|Default|Setref%20to%20player _asplayer_vechile_proto))
  (CallFunction|ChecktoSeeifPlayerUsedMovmentContrals (Math|Boolean|ANDBoolean (Variables|/Game/VehicleAdvBP/Blueprints/Players/PlayerVechilePROTO.PlayerVechilePROTO_C|GetWSmovment _asplayer_vechile_proto) (Variables|/Game/VehicleAdvBP/Blueprints/Players/PlayerVechilePROTO.PlayerVechilePROTO_C|GetHandbrake _asplayer_vechile_proto) (Variables|/Game/VehicleAdvBP/Blueprints/Players/PlayerVechilePROTO.PlayerVechilePROTO_C|GetADmovment _asplayer_vechile_proto) (Variables|/Game/VehicleAdvBP/Blueprints/Players/PlayerVechilePROTO.PlayerVechilePROTO_C|GetCameraMovement _asplayer_vechile_proto)) _output_get))

(event Custom|INIT
  (params (TUT :type Tutorial%20Player%20Manager%20Object%20Reference))
  (Variables|Default|SetRefToParent TUT))

(fn ConstructionScript
  (|CallParentFunction))

(fn ChecktoSeeifPlayerUsedMovmentContrals
  (params (completed? :type Boolean) (ref%20to%20player :type Player%20Vechile%20PROTO%20Object%20Reference))
  (if completed?
    ;[1 1 1] next phase coll
    (Default|CallOverlapptedColl ref%20to%20player)
    (else
      ;[1 1 1] respawn player
      (bind _outactors (Actor|GetAllActorsOfClass "/Game/VehicleAdvBP/Blueprints/Players/SpawnPoints/ParentPlayerSpawnPoint.ParentPlayerSpawnPoint_C"))
      (Transformation|SetActorRelativeTransform ref%20to%20player (Transformation|GetActorTransform (Utilities|Array|Get(acopy) _outactors)) false true)
      (Development|PrintString "respawn with text sayuing retrey"))))