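; Tutorial trigger volume for the re-right phase, checking whether the player vehicle has used its re-right ability before leaving.
; When a PlayerVechilePROTO ends overlap with the collision, its ReWrite flag is tested.
; If unset, the player is teleported to checkpoint pole number 1 with a 180-degree roll, so it respawns flipped and must use the re-right system.
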(event OnComponentEndOverlap(Coll)
  (params (OverlappedComponent :type Primitive%20Component%20Object%20Reference) (OtherActor :type Actor%20Object%20Reference) (OtherComp :type Primitive%20Component%20Object%20Reference) (OtherBodyIndex :type Integer))
  (bind _asplayer_vechile_proto (Utilities|Casting|CastToPlayerVechilePROTO OtherActor))
  (CallFunction|CheckRewrightHasComplete (Variables|/Game/VehicleAdvBP/Blueprints/Players/PlayerVechilePROTO.PlayerVechilePROTO_C|GetReWrite? _asplayer_vechile_proto) _asplayer_vechile_proto))

(fn ConstructionScript
  (|CallParentFunction))

(fn CheckRewrightHasComplete
  (params (finshted? :type Boolean) (player :type Player%20Vechile%20PROTO%20Object%20Reference))
  (if (not finshted?)
    ;[0 0.1871 1] respawn player
    (bind _outactors (Actor|GetAllActorsOfClass "/Game/VehicleAdvBP/assets/TutorialAssets/PoleForCheckPointMarker.PoleForCheckPointMarker_C"))
    (bind _array_element (Utilities|Array|ForEachLoopwithBreak _outactors :!label _label)
      (:LoopBody
        (if (== (Variables|/Game/VehicleAdvBP/assets/TutorialAssets/PoleForCheckPointMarker.PoleForCheckPointMarker_C|GetPoleNumber _array_element) 1)
          (Transformation|SetActorRelativeTransform player (Math|Transform|MakeTransform (.location (Transformation|GetActorTransform _array_element)) (Math|Rotator|MakeRotator 1.8e+02 (.pitch (.rotation (Transformation|GetActorTransform _array_element))) (.yaw (.rotation (Transformation|GetActorTransform _array_element)))) (.scale (Transformation|GetActorTransform player))) false true) ; 180 roll so that the player uses the rewrite system after respawn
          (goto _label Break)
          (else
            (Development|PrintString "do right one")))))))