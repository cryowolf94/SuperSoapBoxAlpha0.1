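; Tutorial manager Blueprint, apparently meant to step the player through movement, re-right and vehicle attachment phases; it is largely unfinished.
; InitMnager runs a setup function that finds phase collision actors by class, then prints an error if the movement one is missing.
; That function's first Sequence branch returns immediately, ahead of the re-right lookup and owner assignment.
; Phase handlers are stubs, SetNextPhase only prints, and observer bindings are disconnected.
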(event Custom|Init%20Mnager
  ;[1 1 1] inti
  (CallFunction|TutorialCollsionComponentsInit true)
  (Utilities|IsValid (Variables|Default|GetMovementPhaseCol)
    (:Is%20Not%20Valid
      (Development|PrintString "prob"))))

(event Custom|SetNextPhase
  (Development|PrintString "set next phase turn on and off col sections"))

(fn ConstructionScript)

(fn HandleMoveMentPhaseObserver)

(fn HandleReWrite)

(fn HandleRocketAttachmentPhase
  (if true
    _))

(fn TutorialCollsionComponentsInit
  (params (init :type Boolean))
  (if init
    (Utilities|FlowControl|Sequence
      (:then_0
        (bind _outactors (Actor|GetAllActorsOfClass "/Game/VehicleAdvBP/Blueprints/TutorialBP/MovmentPhaseCol1.MovmentPhaseCol1_C"))
        (bind _output_get (Variables|Default|SetMovementPhaseCol (Utilities|Array|Get(acopy) _outactors)))
        (return _output_get))
      (:then_1
        (bind _outactors_2 (Actor|GetAllActorsOfClass "/Game/VehicleAdvBP/Blueprints/TutorialBP/RerightPhaseCol2.RerightPhaseCol2_C"))
        (bind _output_get_2 (Variables|Default|SetRewrightPhase (Utilities|Array|Get(acopy) _outactors_2)))
        (Actor|SetOwner _output_get_2 self))
      (:then_3
        (Actor|GetAllActorsOfClass 0))
      (:then_4
        _)
      (:then_5
        _))
    (return (Variables|Default|GetMovementPhaseCol))
    (else
      (switch int 0))))

(fn HandleGliderAttachmentPhase)

(fn HandleExplosionAttachmentPhase)

(fn GetColl
  (params (ActorClass :type Tutorial%20Player%20Manager%20Class%20Reference))
  (bind _outactors (Actor|GetAllActorsOfClass ActorClass))
  (return _outactors))